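; BP_Spawner is an enemy spawner that keeps a tracked population of up to ten BP_Enemy actors around itself.
; While the count is below the cap, a Delay on Tick throttles spawning at random navigable points within a radius of the spawner.
; A DoOnce reset by a one-second Delay periodically removes dead enemies from the array during iteration, freeing slots for replacements.
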(event EventTick
  (params (DeltaSeconds :type Float%20%28single-precision%29))
  (bind _enemies (Variables|Default|GetEnemies))
  (Utilities|FlowControl|Sequence
    (:then_0
      (if (< (Utilities|Array|Length (Variables|Default|GetEnemies)) 10)
        (Utilities|FlowControl|Delay 0.2)
        (bind _randomlocation (Class|NavigationSystemV1|GetRandomLocationinNavigableRadius (Transformation|GetActorLocation) 1.25e+03 0 0))
        (bind _returnvalue (Game|SpawnActorfromClass "/Game/Blueprints/Enemy/BP_Enemy.BP_Enemy_C" (Math|Conversions|ToTransform(Vector) _randomlocation) "Undefined" 0 0))
        (Utilities|Array|Add (Variables|Default|GetEnemies) _returnvalue)))
    (:then_1
      (Utilities|FlowControl|DoOnce false :!label _label
        (:Completed
          (for _array_element _enemies
            (if (Variables|/Game/Blueprints/Enemy/BP_Enemy.BP_Enemy_C|GetIsDead _array_element)
              (Utilities|Array|RemoveItem _enemies _array_element)))
          (Utilities|FlowControl|Delay 1.0)
          (goto _label Reset))))))

(fn ConstructionScript)