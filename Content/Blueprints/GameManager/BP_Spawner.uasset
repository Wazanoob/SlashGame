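; BP_Spawner manages the enemy encounter: it spawns waves of BP_Enemy, starts the boss battle and handles victory music.
; Tick keeps up to six enemies alive at random navigable points around the spawner until a spawn count cap is reached.
; When one enemy remains, StartBossBattle swaps music, plays the Boss roar and destroys pre-fight actors.
; Once none remain, the music mutes and a victory sound plays; a timeline volume fade is left unconnected.
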(event Custom|StartBossBattle
  (bind _backgroundmusic (Variables|Default|GetBackgroundMusic))
  (Audio|Components|Audio|SetSound _backgroundmusic "/Game/Sound/Music/BossMusic.BossMusic")
  (Audio|Components|Audio|Play _backgroundmusic 0.35)
  (Audio|Components|Audio|AdjustVolume _backgroundmusic 0.0 0.5 "Linear" :!class /Script/Engine.AudioComponent)
  (Animation|PlayAnimMontage (Variables|Default|GetBoss) "/Game/Animation/Enemy/AM_Roar_Monster.AM_Roar_Monster" 1.0 "None")
  (for _array_element (Variables|Default|GetActorsPreFight)
    (Actor|DestroyActor _array_element))
  (Variables|Default|SetBossBattleStarted true))

(event EventBeginPlay
  (Utilities|FlowControl|Sequence
    (:then_0
      (bind _returnvalue (Audio|SpawnSoundAttached "/Game/Sound/Music/BackgroundMusic.BackgroundMusic" (Variables|Default|GetMusic) "None" "0, 0, 0" "0, 0, 0" "KeepRelativeOffset" false 0.1 1.0 0.0 0 0 false))
      (Variables|Default|SetBackgroundMusic _returnvalue))))

(event EventTick
  (params (DeltaSeconds :type Float%20%28single-precision%29))
  (Utilities|FlowControl|Sequence
    (:then_0
      (bind _outactors (Actor|GetAllActorsOfClass "/Game/Blueprints/Enemy/BP_Enemy.BP_Enemy_C"))
      (if (and (< (Utilities|Array|Length _outactors) 6) (<= (Variables|Default|GetEnemyCount) 8))
        (Utilities|FlowControl|Delay 0.4)
        (bind _randomlocation (Class|NavigationSystemV1|GetRandomLocationinNavigableRadius (Transformation|GetActorLocation) 1.25e+03 0 0))
        (bind _returnvalue (Game|SpawnActorfromClass "/Game/Blueprints/Enemy/BP_Enemy.BP_Enemy_C" (Math|Conversions|ToTransform(Vector) _randomlocation) "Undefined" 0 0))
        (if (Utilities|IsValid _returnvalue)
          (bind _result (Math|Integer|IncrementInt (Variables|Default|GetEnemyCount))
            (:%20%20
              (Development|PrintString (Utilities|String|ToString(Integer) _result)))))
        (elif (and (== (Utilities|Array|Length _outactors) 1) (>= (Variables|Default|GetEnemyCount) 8))
          (Utilities|FlowControl|DoOnce false
            (:Completed
              (CallFunction|StartBossBattle))))))
    (:then_1
      (if (Variables|Default|GetBossBattleStarted)
        (bind _outactors_2 (Actor|GetAllActorsOfClass "/Game/Blueprints/Enemy/BP_Enemy.BP_Enemy_C"))
        (if (== (Utilities|Array|Length _outactors_2) 0)
          (Utilities|FlowControl|DoOnce false
            (:Completed
              (Audio|Components|Audio|AdjustVolume (Variables|Default|GetBackgroundMusic) 0.0 0.0 "Linear" :!class /Script/Engine.AudioComponent)
              (Audio|PlaySound2D "/Game/Sound/EventSound/VictorySound.VictorySound" 0.2 1.0 0.0 0 0))))))))

(fn ConstructionScript)