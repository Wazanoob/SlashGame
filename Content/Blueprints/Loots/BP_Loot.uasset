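; BP_Loot is a loot actor that plays a spawn animation before revealing its widget.
; On BeginPlay it hides the widget, stores its starting location and plays a timeline.
; The timeline's ZAxis track offsets the height from that start point, while its Rotation track drives roll and pitch with yaw held fixed.
; The widget becomes visible when the timeline finishes.
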(event EventBeginPlay
  (Utilities|FlowControl|Sequence
    (:then_0
      (Development|SetHiddeninGame (Variables|Default|GetWidget) true false))
    (:then_1
      (Variables|Default|SetNewVar (Transformation|GetActorLocation))
      (bind (_direction _z_axis _rotation) (Timeline|Timeline PlayFromStart)
        (:Update
          (Transformation|SetActorLocation (Math|Vector|MakeVector (.x (Variables|Default|GetNewVar)) (.y (Variables|Default|GetNewVar)) (+ (.z (Variables|Default|GetNewVar)) (* _z_axis 2.0))) false false)
          (Transformation|SetActorRotation (Math|Rotator|MakeRotator (* _rotation 1.0) (* _rotation 1.0) -9e+01)))
        (:Finished
          (Development|SetHiddeninGame (Variables|Default|GetWidget) false false))))))

(fn ConstructionScript)