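; BP_Soul is a loot actor that flies from its starting location to the player, then destroys itself.
; BeginPlay stores the start location, and a DoOnce on the first Tick starts the SmoothMove timeline.
; Each update interpolates by the SmoothDamp curve toward player 0's current pawn location, so it follows a moving player, without sweep.
; No reward or pickup effect is applied in this Blueprint.
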(event EventTick
  (params (DeltaSeconds :type Float%20%28single-precision%29))
  (bind _startlocation (Variables|Default|GetStartLocation))
  (Utilities|FlowControl|DoOnce false
    (:Completed
      (bind _smoothdamp (Timeline|SmoothMove PlayFromStart)
        (:Update
          (Transformation|SetActorLocation (+ (* (- (Transformation|GetActorLocation (Game|Player|GetPlayerPawn 0)) _startlocation) _smoothdamp) _startlocation) false false))
        (:Finished
          (Actor|DestroyActor))))))

(event EventBeginPlay
  (Variables|Default|SetStartLocation (Transformation|GetActorLocation)))

(fn ConstructionScript)