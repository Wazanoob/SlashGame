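; Zombie enemy character that takes hits, shows a name and life bar widget, and dies leaving a soul pickup actor behind.
; GetHit, throttled by a DoOnce that resets after 0.2 seconds, plays a reaction montage and sound, launches the enemy, subtracts life and updates the bar.
; At zero life, Die disables collision, hides the widget and plays a death montage whose notify spawns BP_Soul and destroys the actor.
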(event Custom|Enable/Disable%20Widget
  (params (IsEnable :type Boolean))
  (bind _widget (Variables|Default|GetWidget))
  ;[0 0.2479 1] Hide / Unhide character info
  (if IsEnable
    (Development|SetHiddeninGame _widget false false)
    (else
      (Development|SetHiddeninGame _widget true false))))

(event Custom|UpdateLifeBar
  ;[0 0.2479 1] Update Life bar
  (bind _asbpw_target (Utilities|Casting|CastToBPW_Target (UserInterface|GetWidget (Variables|Default|GetWidget))))
  (bind _result (Math|Float|DecrementFloat (/ (Variables|CharacterStats|GetCurrentLife) (Variables|CharacterStats|GetMaxLife)))
    (:%20%20
      (Default|SetLifeBar _asbpw_target (Math|Float|Absolute(Float) _result)))))

(event Custom|Die
  (bind _capsulecomponent (Variables|Collision|GetCapsuleComponent))
  ;[0 0.2479 1] Death
  (Variables|Default|SetIsDead true)
  (Collision|SetCollisionResponsetoChannel _capsulecomponent "ECC_Visibility" "ECR_Ignore")
  (Collision|SetCollisionResponsetoChannel _capsulecomponent "ECC_Pawn" "ECR_Ignore")
  (Collision|SetCollisionEnabled (Variables|Character|GetMesh) "NoCollision")
  (CallFunction|Enable/DisableWidget false)
  (Animation|Montage|PlayMontage (Variables|Character|GetMesh) "/Game/Animation/Enemy/AM_Death.AM_Death"
    (:OnNotifyBegin
      (Game|SpawnActorfromClass "/Game/Blueprints/Loots/BP_Soul.BP_Soul_C" (Math|Conversions|ToTransform(Vector) (+ (Transformation|GetActorLocation) "0,0,50.000000")) "Undefined" 0 0)
      (Actor|DestroyActor))))

(event EventBeginPlay
  (bind _widget (Variables|Default|GetWidget))
  ;[1 1 1] BEGIN PLAY
  (Utilities|FlowControl|Sequence
    (:then_0
      ;[0 0.2479 1] Hide widget & set current life at begin play
      (Development|SetHiddeninGame _widget true false)
      (bind _asbpw_target (Utilities|Casting|CastToBPW_Target (UserInterface|GetWidget _widget)))
      (Default|SetTextName _asbpw_target "Zombie")
      (Default|SetLifeBar _asbpw_target 0.0))
    (:then_1
      (Variables|CharacterStats|SetCurrentLife (Variables|CharacterStats|GetMaxLife)))))

(event EventGetHit
  (params (Direction :type Vector :default "0, 0, 0") (DamageAmount :type Integer))
  (bind _mesh (Variables|Character|GetMesh))
  (bind _returnvalue (Components|SkeletalMesh|GetAnimInstance _mesh))
  ;[0 0.2479 1] Get hit
  (Utilities|FlowControl|DoOnce false :!label _label
    (:Completed
      (Utilities|FlowControl|Sequence
        (:then_0
          (Animation|Montage|MontagePlay _returnvalue "/Game/Animation/Enemy/AM_HitReaction.AM_HitReaction" 1.0 "MontageLength" 0.0 true)
          (Ability|Animation|MontageJumptoSection _returnvalue "Back" "/Game/Animation/Enemy/AM_HitReaction.AM_HitReaction")
          (Character|LaunchCharacter (* Direction (Variables|Default|GetLaunchVelocity)) false false)
          (Audio|PlaySoundatLocation "/Game/Sound/HitSound/Flesh/sfx_HitFlesh.sfx_HitFlesh" (Transformation|GetActorLocation) "0, 0, 0" 1.0 1.0 0.0 0 0 0 0)
          (Utilities|FlowControl|Delay 0.2)
          (goto _label Reset))
        (:then_1
          (Variables|CharacterStats|SetCurrentLife (- (Variables|CharacterStats|GetCurrentLife) DamageAmount))
          (CallFunction|UpdateLifeBar))
        (:then_2
          (if (<= (Variables|CharacterStats|GetCurrentLife) 0)
            (CallFunction|Die)))))))

(fn ConstructionScript)