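; Boss enemy "Big Boy" that sets up its target widget and handles its own death sequence.
; BeginPlay hides and initializes the name and life bar widget, resets life to max and applies materials.
; Die disables mesh collision, makes the capsule ignore Visibility and Pawn, and plays a death montage whose notify destroys the actor.
; While dead, Tick drifts it forward and up by a fixed per-frame offset, unscaled by delta time.
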(event EventBeginPlay
  (bind _widget (Variables|Default|GetWidget))
  (Utilities|FlowControl|Sequence
    (:then_0
      (Development|SetHiddeninGame _widget true false)
      (bind _asbpw_target (Utilities|Casting|CastToBPW_Target (UserInterface|GetWidget _widget)))
      (Default|SetTextName _asbpw_target "Big Boy")
      (Default|SetLifeBar _asbpw_target 0.0))
    (:then_1
      (Variables|Default|SetCurrentLife (Variables|Default|GetMaxLife)))
    (:then_2
      (CallFunction|SetMaterials))))

(event EventTick
  (params (DeltaSeconds :type Float%20%28single-precision%29))
  (if (Variables|Default|GetIsDead)
    (Transformation|AddActorWorldOffset (+ (Transformation|GetActorForwardVector) "0,0,1.000000"))))

(event EventDie
  (bind _capsulecomponent (Variables|Default|GetCapsuleComponent))
  (Variables|Default|SetIsDead true)
  (Collision|SetCollisionResponsetoChannel _capsulecomponent "ECC_Visibility" "ECR_Ignore")
  (Collision|SetCollisionResponsetoChannel _capsulecomponent "ECC_Pawn" "ECR_Ignore")
  (Collision|SetCollisionEnabled (Variables|Character|GetMesh) "NoCollision")
  (CallFunction|Enable/DisableWidget false)
  (Animation|Montage|PlayMontage (Variables|Character|GetMesh) (Variables|Default|GetDeathMontage)
    (:OnNotifyBegin
      (Actor|DestroyActor))))

(fn ConstructionScript)