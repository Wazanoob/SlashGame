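; Player melee weapon that attaches to the character's weapon socket and drives a First Ability combo attack.
; Input plays the combo montage with movement frozen, while presses during it buffer an index that montage notifies check to stop, continue or chain into a power attack.
; Hitbox overlaps run a box trace, send hit direction through BPI_Hit and spawn blood at the impact point.
; An unconnected branch would randomize the power attack section.
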(event OnComponentBeginOverlap(Box)
  (params (OverlappedComponent :type Primitive%20Component%20Object%20Reference) (OtherActor :type Actor%20Object%20Reference) (OtherComp :type Primitive%20Component%20Object%20Reference) (OtherBodyIndex :type Integer) (bFromSweep :type Boolean) (SweepResult :type Hit%20Result%20Structure%20%28by%20ref%29))
  ;[1 1 1] Hit impact location
  (bind _outhit (Collision|BoxTraceByChannel (Transformation|GetWorldLocation (Variables|Default|GetStart)) (Transformation|GetWorldLocation (Variables|Default|GetEnd)) "20.000000,20.000000,20.000000" "0, 0, 0" "TraceTypeQuery1" false 0 "None"))
  (if (Utilities|DoesObjectImplementInterface (.hitactor _outhit) "/Game/Blueprints/Weapons/BPI_Hit.BPI_Hit_C")
    (Class|BPIHit|GetHit(Message) (.hitactor _outhit) (Math|Vector|GetUnitDirection(Vector) (Transformation|GetActorLocation (Game|Player|GetPlayerPawn 0)) (Transformation|GetActorLocation (.hitactor _outhit))))
    (Effects|SpawnEmitteratLocation "/Game/Realistic_Starter_VFX_Pack_Vol2/Particles/Blood/P_Blood_Splat_Cone.P_Blood_Splat_Cone" (.impactpoint _outhit) "0, 0, 0" "0.600000,0.600000,0.600000")))

(event Input|EnhancedActionEvents|EnhancedInputActionIA_FirstAbility
  (params (ActionValue :type Boolean) (ElapsedSeconds :type Float%20%28double-precision%29) (TriggeredSeconds :type Float%20%28double-precision%29) (InputAction :type Input%20Action%20Object%20Reference :default "/Game/Inputs/IA_FirstAbility.IA_FirstAbility"))
  (bind _animinstance (Variables|PlayerReferences|GetAnimInstance))
  ;[1 1 1] First Ability input
  (:Triggered
    (if (not (Animation|Montage|MontageIsPlaying _animinstance "/Game/Animation/Player/AM_Combot.AM_Combot"))
      (if (not (Class|AnimInstance|IsAnyMontagePlaying _animinstance))
        (Default|Freeze/UnfreezeMovement (Variables|PlayerReferences|GetPlayer) true)
        (Animation|Montage|PlayMontage (Variables|Default|GetPlayerMesh) "/Game/Animation/Player/AM_Combot.AM_Combot"
          (:OnNotifyBegin
            (bind _result (Math|Integer|DecrementInt (Variables|PlayerReferences|GetFirstAbilityIndex))
              (:%20%20
                (if (< _result 0)
                  (Animation|Montage|MontageStop (Variables|PlayerReferences|GetAnimInstance) 0.3 "/Game/Animation/Player/AM_Combot.AM_Combot")
                  (Variables|PlayerReferences|SetFirstAbilityIndex 0)
                  (Default|Freeze/UnfreezeMovement (Variables|PlayerReferences|GetPlayer) false :!label _label)
                  (else
                    (Default|ForceSetPlayerRotation (Variables|PlayerReferences|GetPlayer)))))))
          (:OnNotifyEnd
            (bind _result_2 (Math|Integer|DecrementInt (Variables|PlayerReferences|GetFirstAbilityIndex))
              (:%20%20
                (if (< _result_2 0)
                  (goto _label)
                  (else
                    (Animation|Montage|MontageStop (Variables|PlayerReferences|GetAnimInstance) 0.3 "/Game/Animation/Player/AM_Combot.AM_Combot")
                    (Default|ForceSetPlayerRotation (Variables|PlayerReferences|GetPlayer))
                    (Animation|Montage|PlayMontage (Variables|Default|GetPlayerMesh) "/Game/Animation/Player/AM_PowerAttack.AM_PowerAttack" 1.0 0.0 "1"
                      (:then
                        (Variables|PlayerReferences|SetFirstAbilityIndex 0))
                      (:OnNotifyBegin
                        (Animation|Montage|MontageStop (Variables|PlayerReferences|GetAnimInstance) 0.3 "/Game/Animation/Player/AM_PowerAttack.AM_PowerAttack")
                        (Default|Freeze/UnfreezeMovement (Variables|PlayerReferences|GetPlayer) false))))))))))
      (else
        (Variables|PlayerReferences|SetFirstAbilityIndex 1)))))

(event EventBeginPlay
  ;[1 1 1] Set player references
  (Utilities|FlowControl|Sequence
    (:then_0
      (bind _asbp_player_character (Utilities|Casting|CastToBP_PlayerCharacter (Game|Player|GetPlayerPawn 0)))
      (bind _output_get (Variables|PlayerReferences|SetPlayer _asbp_player_character))
      (Variables|Default|SetPlayerMesh (Variables|/Script/Engine.Character|GetMesh _output_get))
      (Variables|PlayerReferences|SetAnimInstance (Components|SkeletalMesh|GetAnimInstance (Variables|/Script/Engine.Character|GetMesh _output_get))))
    (:then_1
      (Transformation|AttachComponentToComponent (Variables|Default|GetWeapon) (Variables|/Script/Engine.Character|GetMesh (Variables|PlayerReferences|GetPlayer)) "Socket_Weapon" "SnapToTarget" "SnapToTarget" "SnapToTarget" true))))

(fn ConstructionScript)